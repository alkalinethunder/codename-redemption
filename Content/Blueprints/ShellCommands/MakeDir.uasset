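; MakeDir is an in-game shell command that creates a directory in the game's file system.
; On Run, it joins its arguments without a separator, converts the result to an absolute path and passes it to the file system's MakeDirectory.
; If that call fails, it writes an error with the command name and path to the console, stating that the file or directory exists.
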(event `self.Run`
  (bind _returnvalue (`self.RelativeToAbsolutePath` (`KismetStringLibrary.JoinStringArray` (`self.GetArguments`))))
  (bind _returnvalue_2 (`VirtualFileSystem.MakeDirectory` (`self.GetFileSystem`) _returnvalue))
  (if (not _returnvalue_2)
    (`ConsoleWidget.WriteLine` (`self.GetConsole`) (`KismetTextLibrary.Conv_StringToText` (`KismetStringLibrary.Concat_StrStr` (`self.GetCommandName`) ": " _returnvalue ": File or directory exists.")))))