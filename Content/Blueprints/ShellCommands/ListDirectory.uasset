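; Shell command Blueprint that lists the child directories of the working path in an in-game console.
; Its Run event queries the file system for child directory paths and writes each one as its own console line.
; If the query fails, it writes a "Directory not found." error that includes the command name and working path.
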(event `self.Run`
  (bind _returnvalue (`self.GetWorkingPath`))
  (bind _returnvalue_2 (`self.GetConsole`))
  (bind (_outchildren _returnvalue_3) (`VirtualFileSystem.GetChildDirectoryPaths` (`self.GetFileSystem`) _returnvalue))
  (if _returnvalue_3
    (for _array_element _outchildren
      (`ConsoleWidget.WriteLine` _returnvalue_2 (`KismetTextLibrary.Conv_StringToText` _array_element)))
    (else
      (`ConsoleWidget.WriteLine` _returnvalue_2 (`KismetTextLibrary.Conv_StringToText` (`KismetStringLibrary.Concat_StrStr` (`self.GetCommandName`) ": " _returnvalue ": Directory not found."))))))