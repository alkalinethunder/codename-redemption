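; Tracert is a shell command Blueprint that prints the network route from the player's network to a given hostname or IP address in the in-game console.
; On Run it joins and trims the arguments, resolves the address through the network manager, then calls TraceRoute on its own network.
; Each hop prints as hostname and IP, while an empty argument or unresolvable address prints an error prefixed with the command name.
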(event `self.Run`
  (bind (_outnetwork _returnvalue) (`NetworkManager.ResolveNetworkAddress` (`self.GetNetworkManager`) (`self.IP`)))
  ;[1 1 1] Retrieve the specified IP address from the user and check if it was empty or not.
  (bind _output_get (set `self.IP` (`KismetStringLibrary.Trim` (`KismetStringLibrary.JoinStringArray` (`self.GetArguments`)))))
  (if (`KismetStringLibrary.IsEmpty` _output_get)
    ;[1 1 1] Print the "hostname required" error.
    (`ConsoleWidget.WriteLine` (`self.GetConsole`) (`KismetTextLibrary.Conv_StringToText` (`KismetStringLibrary.Concat_StrStr` (`self.GetCommandName`) ": hostname or IP address required.")))
    (else
      ;[1 1 1] Try to resolve the given IP to a network node.
      (if _returnvalue
        (bind _returnvalue_2 (`NetworkNode.TraceRoute` (`self.GetMyNetwork`) _outnetwork))
        (for _array_element _returnvalue_2
          (`ConsoleWidget.WriteLine` (`self.GetConsole`) (`KismetTextLibrary.Conv_StringToText` (`KismetStringLibrary.Concat_StrStr` (`NetworkNode.GetHostName` _array_element) " (" (`NetworkNode.GetIPAddress` _array_element) ")"))))
        (else
          ;[1 1 1] Network unreachable...
          (`ConsoleWidget.WriteLine` (`self.GetConsole`) (`KismetTextLibrary.Conv_StringToText` (`KismetStringLibrary.Concat_StrStr` (`self.GetCommandName`) ": " (`self.IP`) ": Network unreachable."))))))))