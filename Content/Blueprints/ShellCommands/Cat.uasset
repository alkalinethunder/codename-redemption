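; Shell command Blueprint for "cat", which prints a file's text to the in-game console.
; On Run it joins all arguments with no separator into one path and resolves it against the working directory.
; It reads that path through the file system and writes the text to the console.
; A failed read prints a "File not found" error built from the command name and the read's OutText, not the path.
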(event `self.Run`
  (bind (_outtext _returnvalue) (`VirtualFileSystem.GetFileTextIfFileExists` (`self.GetFileSystem`) (`PathUtils.GetAbsolutePath` (`self.GetWorkingPath`) (`KismetStringLibrary.JoinStringArray` (`self.GetArguments`)))))
  ;[1 1 1] Try to read the specified file's text.
  (if _returnvalue
    ;[1 1 1] If it worked, write it to the console.
    (`ConsoleWidget.WriteLine` (`self.GetConsole`) (`KismetTextLibrary.Conv_StringToText` _outtext))
    (else
      ;[1 1 1] If that didn't work, print a file not found error.
      (`ConsoleWidget.WriteLine` (`self.GetConsole`) (`KismetTextLibrary.Conv_StringToText` (`KismetStringLibrary.Concat_StrStr` (`self.GetCommandName`) ": " _outtext ": File not found."))))))