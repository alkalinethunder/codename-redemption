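; GuiFunctions is a Blueprint function library of shared UI helpers for icon buttons and modal windows.
; MakeIconButtonStyle builds a button style from one icon, tinted per idle, hovered, pressed and disabled state, and SetButtonStyleToIcon applies it to a button.
; SpawnModal creates a ModalHost with a title and icon, adds it to the viewport, then places the given widget in its content slot.
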(fn `Make Icon Button Style`
  (params (Icon :type "Texture2D Object Reference"))
  (returns (`Button Style` :type "ButtonStyle Structure"))
  (locals (`Idle Tint` :type "SlateColor Structure" :default (struct :`SpecifiedColor` (struct :`R` 1.0 :`G` 1.0 :`B` 1.0 :`A` 1.0) :`ColorUseRule` "UseColor_Specified")) (`Disabled Tint` :type "SlateColor Structure" :default (struct :`SpecifiedColor` (struct :`R` 0.215861 :`G` 0.215861 :`B` 0.215861 :`A` 1.0) :`ColorUseRule` "UseColor_Specified")) (`Pressed Tint` :type "SlateColor Structure" :default (struct :`SpecifiedColor` (struct :`R` 0.006935 :`G` 0.254357 :`B` 0.588542 :`A` 1.0) :`ColorUseRule` "UseColor_Specified")) (`Hovered Tint` :type "SlateColor Structure" :default (struct :`SpecifiedColor` (struct :`R` 0.01096 :`G` 0.401978 :`B` 0.930111 :`A` 1.0) :`ColorUseRule` "UseColor_Specified")))
  (return (make `ButtonStyle` (make `SlateBrush` (24.0 24.0) (struct) (`local.Idle Tint`) Icon) (make `SlateBrush` (24.0 24.0) (struct) (`local.Hovered Tint`) Icon) (make `SlateBrush` (24.0 24.0) (struct) (`local.Pressed Tint`) Icon) (make `SlateBrush` (24.0 24.0) (struct) (`local.Disabled Tint`) Icon))))

(fn `Set Button Style to Icon`
  (params (Button :type "Button Object Reference") (Icon :type "Texture2D Object Reference"))
  (`Button.SetStyle` Button (`self.Make Icon Button Style` Icon Button)))

(fn `Spawn Modal`
  (params (`In Widget` :type "UserWidget Object Reference") (`Owning Player` :type "PlayerController Object Reference") (`Title Text` :type Text) (`Title Icon` :type "Texture2D Object Reference"))
  (bind _returnvalue (`|CreateWidget` "/Game/Gui/Components/ModalHost.ModalHost_C" `Owning Player` `Title Text` `Title Icon`))
  (`UserWidget.AddToViewport` _returnvalue 0)
  (`/Game/Gui/Components/ModalHost.Set Content Slot Widget` _returnvalue `In Widget`))